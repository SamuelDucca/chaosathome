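; BP_ImpactDamage is a short-lived Chaos field actor that damages and scatters destructible structures at an impact point.
; On BeginPlay it applies external cluster strain through a radial falloff, scaling magnitude and radius with ImpactForce around its sphere component.
; It then adds angular and linear velocity as radial vectors multiplied by linear falloff, also scaled by impact force.
; The actor destroys itself after a brief delay.
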(event `self.ReceiveBeginPlay`
  (bind _sphere (`self.Sphere`))
  (bind _sphere_2 (`self.Sphere`))
  (bind _sphere_3 (`self.Sphere`))
  ;[1 1 1] Apply strain on structure based on impact force
  (`FieldSystemComponent.ApplyPhysicsField` (`self.FieldSystemComponent`) true "Field_ExternalClusterStrain" null (`RadialFalloff.SetRadialFalloff` (`self.RadialFalloff`) (* (`self.Magnitude`) (`self.ImpactForce`)) 0.0 1.0 0.0 (* (`SphereComponent.SphereRadius` _sphere_3) (+ 1.0 (* (`self.ImpactForce`) 0.2))) (`SceneComponent.K2_GetComponentLocation` _sphere_3) "Field_FallOff_None"))
  ;[1 1 1] Apply Angular Velocity
  (`FieldSystemComponent.ApplyPhysicsField` (`self.FieldSystemComponent`) true "Field_AngularVelociy" null (`OperatorField.SetOperatorField` (`self.OperatorField`) 1.0 (`RadialVector.SetRadialVector` (`self.RadialVector`) (* (`self.ForceMagnitude`) (`self.ImpactForce`)) (`SceneComponent.K2_GetComponentLocation` (`self.Sphere`))) (`RadialFalloff.SetRadialFalloff` (`self.RadialFalloff`) 1.0 0.0 1.0 0.0 (`SphereComponent.SphereRadius` _sphere_2) (`SceneComponent.K2_GetComponentLocation` _sphere_2) "Field_Falloff_Linear") "Field_Multiply"))
  ;[1 1 1] Apply Linear Velocity
  (`FieldSystemComponent.ApplyPhysicsField` (`self.FieldSystemComponent`) true "Field_LinearVelocity" null (`OperatorField.SetOperatorField` (`self.OperatorField`) 1.0 (`RadialVector.SetRadialVector` (`self.RadialVector`) (* (`self.ForceMagnitude`) (`self.ImpactForce`)) (`SceneComponent.K2_GetComponentLocation` (`self.FieldSystemComponent`))) (`RadialFalloff.SetRadialFalloff` (`self.RadialFalloff`) 1.0 0.0 1.0 0.0 (`SphereComponent.SphereRadius` _sphere) (`SceneComponent.K2_GetComponentLocation` _sphere) "Field_Falloff_Linear") "Field_Multiply"))
  (`KismetSystemLibrary.Delay` 0.1)
  (`self.K2_DestroyActor`))

(fn `UserConstructionScript`)