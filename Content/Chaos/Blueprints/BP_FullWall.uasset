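; BP_FullWall is a Chaos destructible wall made of five planks that awards a point once every plank has broken.
; Each plank's break event disables its further break notifications, since Chaos keeps reporting on already broken pieces, and sets that plank's broken flag.
; All five events share a check that prints a debug string and calls AddScoreMessage on the game mode when all flags are true.
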(event `self.Plank1.OnChaosBreakEvent`
  (params (BreakEvent :type "ChaosBreakEvent Structure (by ref)"))
  ;[1 1 1] Add score if all planks were destroyed
  (`GeometryCollectionComponent.SetNotifyBreaks` (`self.Plank1`) false) ; Chaos manda evento de break mesmo em peças já quebradas. Dando unset após primeiro break para evitar receber notificações excessivas
  (bind _output_get (set `self.Plank1Broken` true))
  (`KismetSystemLibrary.PrintString` "break" :!label _label)
  (if (and _output_get (stale `self.Plank2.OnChaosBreakEvent` _output_get) (stale `self.Plank3.OnChaosBreakEvent` _output_get) (stale `self.Plank4.OnChaosBreakEvent` _output_get) (stale `self.Plank5.OnChaosBreakEvent` _output_get))
    (message `/Game/FirstPersonBP/Blueprints/BI_ScoreCount.AddScore` (`GameplayStatics.GetGameMode`) 1)))

(event `self.Plank2.OnChaosBreakEvent`
  (params (BreakEvent :type "ChaosBreakEvent Structure (by ref)"))
  ;[1 1 1] Add score if all planks were destroyed
  (`GeometryCollectionComponent.SetNotifyBreaks` (`self.Plank2`) false)
  (bind _output_get (set `self.Plank2Broken` true))
  (goto _label))

(event `self.Plank3.OnChaosBreakEvent`
  (params (BreakEvent :type "ChaosBreakEvent Structure (by ref)"))
  ;[1 1 1] Add score if all planks were destroyed
  (`GeometryCollectionComponent.SetNotifyBreaks` (`self.Plank3`) false)
  (bind _output_get (set `self.Plank3Broken` true))
  (goto _label))

(event `self.Plank4.OnChaosBreakEvent`
  (params (BreakEvent :type "ChaosBreakEvent Structure (by ref)"))
  ;[1 1 1] Add score if all planks were destroyed
  (`GeometryCollectionComponent.SetNotifyBreaks` (`self.Plank4`) false)
  (bind _output_get (set `self.Plank4Broken` true))
  (goto _label))

(event `self.Plank5.OnChaosBreakEvent`
  (params (BreakEvent :type "ChaosBreakEvent Structure (by ref)"))
  ;[1 1 1] Add score if all planks were destroyed
  (`GeometryCollectionComponent.SetNotifyBreaks` (`self.Plank5`) false)
  (bind _output_get (set `self.Plank5Broken` true))
  (goto _label))

(fn `UserConstructionScript`)